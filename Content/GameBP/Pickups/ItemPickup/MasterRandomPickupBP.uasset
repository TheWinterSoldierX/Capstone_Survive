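; Base random item pickup that the survivor player collects for health packs, keys, intel or quest items.
; Overlapping the sphere highlights the meshes through custom depth, shows a prompt widget and enables input; leaving hides both and blocks pickup.
; The interaction input switches on the RandomItem type, increments the matching counter on the player character, plays a sound and destroys the pickup.
; Nothing in this Blueprint randomizes RandomItem, and its construction script is empty.
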(event OnComponentBeginOverlap(Sphere)
  (params (OverlappedComponent :type Primitive%20Component%20Object%20Reference) (OtherActor :type Actor%20Object%20Reference) (OtherComp :type Primitive%20Component%20Object%20Reference) (OtherBodyIndex :type Integer) (bFromSweep :type Boolean) (SweepResult :type Hit%20Result%20Structure%20%28by%20ref%29))
  (Utilities|Casting|CastToThirdPersonSurvivor OtherActor)
  (Rendering|SetRenderCustomDepth (Variables|Default|GetSkeletalMesh) true)
  (Rendering|SetVisibility (Variables|Default|GetWidget) true false)
  (Variables|Default|SetCanPickup true)
  (Input|EnableInput (Game|GetPlayerController 0)))

(event OnComponentEndOverlap(Sphere)
  (params (OverlappedComponent :type Primitive%20Component%20Object%20Reference) (OtherActor :type Actor%20Object%20Reference) (OtherComp :type Primitive%20Component%20Object%20Reference) (OtherBodyIndex :type Integer))
  (Utilities|Casting|CastToThirdPersonSurvivor OtherActor)
  (Rendering|SetRenderCustomDepth (Variables|Default|GetSkeletalMesh) false)
  (Rendering|SetVisibility (Variables|Default|GetWidget) false false)
  (Variables|Default|SetCanPickup false))

(event Input|ActionEvents|InputActionItemInteraction
  (params (Key :type Key%20Structure))
  (:Pressed
    (if (Variables|Default|GetCanPickup)
      (switch Utilities|FlowControl|Switch|SwitchonRandomPickupType (Variables|Default|GetRandomItem)
        (:NewEnumerator1
          (bind _asthird_person_survivor (Utilities|Casting|CastToThirdPersonSurvivor (Game|GetPlayerCharacter 0)))
          (bind _result (Math|Integer|IncrementInt (Variables|/Game/GameBP/PlayerBlueprints/ThirdPersonSurvivor.ThirdPersonSurvivor_C|GetHealthPack _asthird_person_survivor))
            (:%20%20
              (Variables|/Game/GameBP/PlayerBlueprints/ThirdPersonSurvivor.ThirdPersonSurvivor_C|SetHealthPack _asthird_person_survivor _result)
              (Audio|PlaySound2D "/Game/Assets/MilitaryWeapSilver/Sound/GrenadeLauncher/Cues/GrenadeLauncher_AmmoPickup_Cue.GrenadeLauncher_AmmoPickup_Cue" 1.0 1.0 0.0 0 0)
              (Actor|DestroyActor) ; Destroy it from the Floor
            )))
        (:NewEnumerator2
          (bind _asthird_person_survivor_2 (Utilities|Casting|CastToThirdPersonSurvivor (Game|GetPlayerCharacter 0)))
          (bind _result_2 (Math|Integer|IncrementInt (Variables|/Game/GameBP/PlayerBlueprints/ThirdPersonSurvivor.ThirdPersonSurvivor_C|GetKey _asthird_person_survivor_2))
            (:%20%20
              (Variables|/Game/GameBP/PlayerBlueprints/ThirdPersonSurvivor.ThirdPersonSurvivor_C|SetKey _asthird_person_survivor_2 _result_2)
              (Audio|PlaySound2D "/Game/Assets/MilitaryWeapSilver/Sound/Shotgun/Cues/Shotgun_AmmoPickup_Cue.Shotgun_AmmoPickup_Cue" 1.0 1.0 0.0 0 0)
              (Actor|DestroyActor) ; Destroy it from the Floor
            )))
        (:NewEnumerator3
          (bind _asthird_person_survivor_3 (Utilities|Casting|CastToThirdPersonSurvivor (Game|GetPlayerCharacter 0)))
          (bind _result_3 (Math|Integer|IncrementInt (Variables|/Game/GameBP/PlayerBlueprints/ThirdPersonSurvivor.ThirdPersonSurvivor_C|GetIntel _asthird_person_survivor_3))
            (:%20%20
              (Variables|/Game/GameBP/PlayerBlueprints/ThirdPersonSurvivor.ThirdPersonSurvivor_C|SetIntel _asthird_person_survivor_3 _result_3)
              (Audio|PlaySound2D "/Game/Assets/MilitaryWeapSilver/Sound/Shotgun/Cues/Shotgun_AmmoPickup_Cue.Shotgun_AmmoPickup_Cue" 1.0 1.0 0.0 0 0)
              (Actor|DestroyActor) ; Destroy it from the Floor
            )))
        (:NewEnumerator4
          (bind _asthird_person_survivor_4 (Utilities|Casting|CastToThirdPersonSurvivor (Game|GetPlayerCharacter 0)))
          (bind _result_4 (Math|Integer|IncrementInt (Variables|/Game/GameBP/PlayerBlueprints/ThirdPersonSurvivor.ThirdPersonSurvivor_C|GetQuestItem _asthird_person_survivor_4))
            (:%20%20
              (Variables|/Game/GameBP/PlayerBlueprints/ThirdPersonSurvivor.ThirdPersonSurvivor_C|SetQuestItem _asthird_person_survivor_4 _result_4)
              (Audio|PlaySound2D "/Game/Assets/MilitaryWeapSilver/Sound/Shotgun/Cues/Shotgun_AmmoPickup_Cue.Shotgun_AmmoPickup_Cue" 1.0 1.0 0.0 0 0)
              (Actor|DestroyActor) ; Destroy it from the Floor
            )))))))

(fn ConstructionScript)