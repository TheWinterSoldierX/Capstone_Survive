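; Master weapon pickup that ThirdPersonSurvivor can collect, fire and reload.
; Sphere overlap toggles the prompt widget and custom-depth outline, letting the interaction input pass the weapon to the player's PickUp.
; A gate and retriggerable delay loop automatic fire: camera line traces send random damage and bone name through TakeDamage, while a projectile spawns from the muzzle.
; GunInfo tracks ammo, refilled from reserve by manual or empty-on-release reloads.
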(event OnComponentBeginOverlap(Sphere)
  (params (OverlappedComponent :type Primitive%20Component%20Object%20Reference) (OtherActor :type Actor%20Object%20Reference) (OtherComp :type Primitive%20Component%20Object%20Reference) (OtherBodyIndex :type Integer) (bFromSweep :type Boolean) (SweepResult :type Hit%20Result%20Structure%20%28by%20ref%29))
  (bind _asthird_person_survivor (Utilities|Casting|CastToThirdPersonSurvivor OtherActor))
  (Variables|Default|SetThirdPersonRef _asthird_person_survivor)
  (CallFunction|OnOff/Visibility/CustomDepth true true)
  (Variables|Default|SetCanWePick true)
  (Input|EnableInput (Game|GetPlayerController 0))
  (Physics|SetSimulatePhysics (Variables|Default|GetSkeletalMesh) false))

(event OnComponentEndOverlap(Sphere)
  (params (OverlappedComponent :type Primitive%20Component%20Object%20Reference) (OtherActor :type Actor%20Object%20Reference) (OtherComp :type Primitive%20Component%20Object%20Reference) (OtherBodyIndex :type Integer))
  (bind _asthird_person_survivor (Utilities|Casting|CastToThirdPersonSurvivor OtherActor))
  (Variables|Default|SetThirdPersonRef _asthird_person_survivor)
  (CallFunction|OnOff/Visibility/CustomDepth false false)
  (Variables|Default|SetCanWePick false))

(event Custom|OffAll
  (CallFunction|OnOff/Visibility/CustomDepth false false)
  (Components|DestroyComponent (Variables|Default|GetSphere)))

(event Custom|StartFire
  (bind _thirdpersonref (Variables|Default|GetThirdPersonRef))
  (bind _skeletalmesh (Variables|Default|GetSkeletalMesh))
  (bind _skeletalmesh_2 (Variables|Default|GetSkeletalMesh))
  (bind _returnvalue (Transformation|GetSocketLocation _skeletalmesh "MuzzleFlash"))
  (bind _followcamera (Variables|/Game/GameBP/PlayerBlueprints/ThirdPersonSurvivor.ThirdPersonSurvivor_C|GetFollowCamera _thirdpersonref))
  (bind _returnvalue_2 (Transformation|GetWorldLocation _followcamera))
  (Utilities|FlowControl|Sequence
    (:then_0
      (goto _label Open))
    (:then_1
      (Utilities|FlowControl|Gate true :!label _label
        (:Exit
          (Utilities|FlowControl|Sequence
            (:then_0
              (Utilities|FlowControl|RetriggerableDelay 0.2)
              (goto _label))
            (:then_1
              (if (<= (.CurrentAmmo (Utilities|Struct|BreakItemType (Variables|Default|GetGunInfo))) 0)
                (Development|PrintString "OUT OF AMMO")
                (else
                  (bind (_outhit _returnvalue_3) (Collision|LineTraceByChannel _returnvalue_2 (+ _returnvalue_2 (* (Math|Vector|GetForwardVector _followcamera) 1.5e+04)) "TraceTypeQuery2" false 0 "None"))
                  (if _returnvalue_3
                    _
                    (else
                      _))
                  (Animation|PlayAnimMontage (Variables|Default|GetThirdPersonRef) (Variables|Default|GetPlayFireAnim) 1.0 "None")
                  (Utilities|Struct|SetmembersinItemType (Variables|Default|GetGunInfo) (- (.CurrentAmmo (Utilities|Struct|BreakItemType (Variables|Default|GetGunInfo))) 1))
                  (if (Utilities|DoesObjectImplementInterface (.HitActor (Collision|BreakHitResult _outhit)) "/Game/GameBP/AI-BluePrints/TakeDamage.TakeDamage_C")
                    (Class|TakeDamage|ITakeDamage(Message) (.HitActor (Collision|BreakHitResult _outhit)) (.HitBoneName (Collision|BreakHitResult _outhit)) (Math|Random|RandomFloatinRange 2e+01 35.0)))
                  (Game|SpawnActorfromClass "/Game/GameBP/PickUps/ProjectileBP.ProjectileBP_C" (Math|Transform|MakeTransform _returnvalue (Math|Rotator|FindLookatRotation _returnvalue (Math|Vector|SelectVector (.ImpactPoint (Collision|BreakHitResult _outhit)) (.TraceEnd (Collision|BreakHitResult _outhit)) _returnvalue_3))) "Undefined" 0 0)
                  (Effects|SpawnEmitteratLocation "/Game/MilitaryWeapSilver/FX/P_Impact_Metal_Medium_01.P_Impact_Metal_Medium_01" (.Location (Collision|BreakHitResult _outhit)))
                  (Effects|SpawnEmitterAttached "/Game/MilitaryWeapSilver/FX/P_AssaultRifle_MuzzleFlash.P_AssaultRifle_MuzzleFlash" (Variables|Default|GetSkeletalMesh) "MuzzleFlash" (Transformation|GetSocketLocation _skeletalmesh_2 "MuzzleFlash") (Transformation|GetSocketRotation _skeletalmesh_2 "MuzzleFlash") "1.000000,1.000000,1.000000" "KeepWorldPosition"))))))))))

(event Custom|AutoReload
  (if (== (Utilities|Struct|BreakItemType (Variables|Default|GetGunInfo)) 0)
    (if (== (Utilities|Struct|BreakItemType (Variables|Default|GetGunInfo)) 0)
      (Development|PrintString "Find Ammos") ; You can add sound here as alternative
      (else
        (Variables|Default|SetIsReloading true)
        (CallFunction|Reloading)
        (Utilities|FlowControl|Delay 2.0) ; Reload Anim Time
        (Variables|Default|SetIsReloading false)))))

(event Custom|Reloading
  (bind _guninfo (Variables|Default|GetGunInfo))
  (bind (_clipsize _currentammo) (Utilities|Struct|BreakItemType _guninfo))
  (if (== (Utilities|Struct|BreakItemType (Variables|Default|GetGunInfo)) 0)
    (Development|PrintString "Find Ammos") ; You can add sound here as alternative
    (elif (== _clipsize _currentammo)
      (Development|PrintString "Full Ammo")
      (else
        (bind _output_get (Variables|Default|SetIsReloading true))
        (if _output_get
          (CallFunction|WeaponReload)
          (Utilities|FlowControl|Delay 2.0) ; Reload Anim Time
          (Variables|Default|SetIsReloading false))))))

(event Custom|StopFire
  (bind _thirdpersonref (Variables|Default|GetThirdPersonRef))
  (bind _skeletalmesh (Variables|Default|GetSkeletalMesh))
  (bind _skeletalmesh_2 (Variables|Default|GetSkeletalMesh))
  (bind _returnvalue (Transformation|GetSocketLocation _skeletalmesh "MuzzleFlash"))
  (bind _followcamera (Variables|/Game/GameBP/PlayerBlueprints/ThirdPersonSurvivor.ThirdPersonSurvivor_C|GetFollowCamera _thirdpersonref))
  (bind _returnvalue_2 (Transformation|GetWorldLocation _followcamera))
  (Utilities|FlowControl|Gate true) ; enters at Close
)

(event Custom|WeaponReload
  (bind _guninfo (Variables|Default|GetGunInfo))
  (bind _guninfo_2 (Variables|Default|GetGunInfo))
  (bind _guninfo_3 (Variables|Default|GetGunInfo))
  (bind _guninfo_4 (Variables|Default|GetGunInfo))
  (bind (_clipsize _currentammo) (Utilities|Struct|BreakItemType _guninfo_4))
  (bind (_currentammo_2 _maxammo) (Utilities|Struct|BreakItemType _guninfo))
  (bind _maxammo_2 (Utilities|Struct|BreakItemType _guninfo_3))
  (if (not (Variables|Default|GetCanFire))
    (Animation|PlayAnimMontage (Variables|Default|GetThirdPersonRef) (Variables|Default|GetWeaponReload_Anim) 1.0 "None")
    (if (> (Utilities|Struct|BreakItemType (Variables|Default|GetGunInfo)) 0)
      (Variables|Default|SetNeededAmmo (- _clipsize _currentammo))
      (if (<= _maxammo_2 (Variables|Default|GetNeededAmmo))
        (Utilities|Struct|SetmembersinItemType _guninfo_2 (+ _currentammo_2 _maxammo))
        (Utilities|Struct|SetmembersinItemType _guninfo_2)
        (else
          (Utilities|Struct|SetmembersinItemType _guninfo_2 (- _maxammo_2 (Variables|Default|GetNeededAmmo)))
          (Utilities|Struct|SetmembersinItemType _guninfo_2 (Utilities|Struct|BreakItemType (Variables|Default|GetGunInfo))))))))

(event Custom|DestroySphere
  (Components|DestroyComponent (Variables|Default|GetSphere)))

(event Custom|FirePress
  (Variables|Default|SetCanFire true)
  (if (not (Variables|Default|GetIsReloading))
    (CallFunction|StartFire)))

(event Custom|FireRelease
  (Variables|Default|SetCanFire false)
  (CallFunction|StopFire)
  (CallFunction|AutoReload))

(event EventBeginPlay)

(event Collision|EventActorBeginOverlap
  (params (OtherActor :type Actor%20Object%20Reference)))

(event EventTick
  (params (DeltaSeconds :type Float%20%28single-precision%29)))

(event Input|ActionEvents|InputActionItemInteraction
  (params (Key :type Key%20Structure))
  (:Pressed
    (if (Variables|Default|GetCanWePick)
      (Default|PickUp (Variables|Default|GetThirdPersonRef) self)
      (Audio|PlaySound2D "/Game/MilitaryWeapSilver/Sound/Rifle/Cues/Rifle_AmmoPickup_Cue.Rifle_AmmoPickup_Cue" 1.0 1.0 0.0 0 0))))

(fn ConstructionScript
  (Variables|Default|SetGunInfo (Utilities|Struct|MakeItemType (.itemtype (Variables|Default|GetGunInfo)) (Utilities|GetClass self) (.clipsize (Variables|Default|GetGunInfo)) (.currentammo (Variables|Default|GetGunInfo)) (.maxammo (Variables|Default|GetGunInfo)) (.damage (Variables|Default|GetGunInfo)) (.itemimage (Variables|Default|GetGunInfo)) (.equipsocketname (Variables|Default|GetGunInfo)) (.unequipsocketname (Variables|Default|GetGunInfo)))))

(fn OnOff/Visibility/CustomDepth
  (params (bNewVisibility :type Boolean) (bValue :type Boolean))
  (Rendering|SetVisibility (Variables|Default|GetWidget) bNewVisibility false)
  (Rendering|SetRenderCustomDepth (Variables|Default|GetSkeletalMesh) bValue))