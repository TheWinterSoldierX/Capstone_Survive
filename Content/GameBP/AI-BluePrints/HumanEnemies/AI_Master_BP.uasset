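; Base human enemy AI that detects the player, carries a weapon and handles damage and death.
; PawnSensing or taking damage sets PlayerFound, and AlertSense overlaps spread it from hunting or dead allies, while a forward trace sets Active.
; Headshots deal double damage, and death triggers ragdoll, then a delayed item drop and cleanup.
; The weapon spawns at BeginPlay and flip-flops between back and hand sockets, with holstering clearing PlayerFound.
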(event OnSeePawn(PawnSensing)
  (params (Pawn :type Pawn%20Object%20Reference))
  ;[1 1 1] AI Sense Player
  (Utilities|Casting|CastToThirdPersonSurvivor Pawn)
  (Variables|Default|SetPlayerFound true))

(event OnComponentBeginOverlap(AlertSense)
  (params (OverlappedComponent :type Primitive%20Component%20Object%20Reference) (OtherActor :type Actor%20Object%20Reference) (OtherComp :type Primitive%20Component%20Object%20Reference) (OtherBodyIndex :type Integer) (bFromSweep :type Boolean) (SweepResult :type Hit%20Result%20Structure%20%28by%20ref%29))
  ;[1 1 1] AI Sense Player
  (if (not (Variables|Default|GetPlayerFound))
    (Utilities|ActiveSense OtherActor)))

(event OnComponentEndOverlap(AlertSense)
  (params (OverlappedComponent :type Primitive%20Component%20Object%20Reference) (OtherActor :type Actor%20Object%20Reference) (OtherComp :type Primitive%20Component%20Object%20Reference) (OtherBodyIndex :type Integer))
  ;[1 1 1] AI Sense Player
  (if (not (Variables|Default|GetPlayerFound))
    (Utilities|ActiveSense OtherActor)))

(event Custom|ScanForPlayer
  (bind _vision_directionarrow (Variables|Default|GetVision%20DirectionArrow))
  (bind _returnvalue (Transformation|GetWorldLocation _vision_directionarrow))
  ;[1 1 1] Scan For Player
  (bind (_outhit _returnvalue_2) (Collision|LineTraceByChannel _returnvalue (+ _returnvalue (* (Math|Vector|GetForwardVector _vision_directionarrow) 2e+03)) "TraceTypeQuery1" true (Utilities|Array|MakeArray self) "None")) ; set none to disable debug lines
  (if _returnvalue_2
    (if (Utilities|DoesObjectImplementInterface (.HitActor (Collision|BreakHitResult _outhit)) "/Game/GameBP/AI-BluePrints/TakeDamage.TakeDamage_C")
      (Utilities|Casting|CastToThirdPersonSurvivor (.HitActor (Collision|BreakHitResult _outhit)))
      (Variables|Default|SetActive true)
      (else
        (Variables|Default|SetActive false)))))

(event Custom|SpawnAIWeapon
  ;[1 1 1] Spawning AI Weapon
  (bind _returnvalue (Game|SpawnActorfromClass (Variables|Default|GetWeaponClass) (Transformation|GetWorldTransform (Variables|Default|GetSphere)) "Undefined" 0 0))
  (bind _output_get (Variables|Default|SetWeaponBP _returnvalue))
  (Transformation|AttachComponentToComponent _output_get (Variables|Character|GetMesh) "Back" "KeepWorld" "KeepWorld" "KeepWorld" true)
  (Default|DestroySphere _output_get))

(event Custom|SpawnItem
  ;[1 1 1] Item Drop From Enemy on Kill
  (switch Utilities|FlowControl|Switch|SwitchonRandomPickupType (Variables|Default|GetRandomItem)
    (:NewEnumerator1
      (Variables|Default|SetItemClass "/Game/GameBP/Pickups/ItemPickup/Health_BP.Health_BP_C"))
    (:NewEnumerator2
      (Variables|Default|SetItemClass "/Game/GameBP/Pickups/ItemPickup/Key_BP.Key_BP_C"))
    (:NewEnumerator3
      (Variables|Default|SetItemClass "/Game/GameBP/Pickups/ItemPickup/Intel_BP.Intel_BP_C"))
    (:NewEnumerator4
      (Variables|Default|SetItemClass "/Game/GameBP/Pickups/ItemPickup/QuestItem_BP.QuestItem_BP_C")))
  (bind _returnvalue (Game|SpawnActorfromClass (Variables|Default|GetItemClass) (Math|Transform|MakeTransform (.Location (Math|Transform|BreakTransform (Transformation|GetSocketTransform (Variables|Character|GetMesh) "pelvis" "RTS_World")))) "Undefined" 0 0))
  (Physics|SetSimulatePhysics (Variables|/Game/GameBP/Pickups/ItemPickup/MasterItemBP.MasterItemBP_C|GetSkeletalMesh _returnvalue) true))

(event Custom|Equip/UnequipWeapon
  ;[1 1 1] Equip/Unequip Weapon
  (Animation|PlayAnimMontage "/Game/Animations/RifleAnimsetPro/Animations/InPlace/EquipRifle_Montage.EquipRifle_Montage" 1.0 "None"))

(event Custom|Equip/Unequip
  ;[1 1 1] Equip/Unequip Weapon
  (Utilities|FlowControl|FlipFlop
    (:A
      (Transformation|AttachComponentToComponent (Variables|Default|GetWeaponBP) (Variables|Character|GetMesh) "GunHold" "KeepRelative" "KeepRelative" "KeepRelative" true)
      (Variables|Default|SetEquipWeapon true))
    (:B
      (Transformation|AttachComponentToComponent (Variables|Default|GetWeaponBP) (Variables|Character|GetMesh) "Back" "KeepRelative" "KeepRelative" "KeepRelative" true)
      (Variables|Default|SetEquipWeapon false)
      (Variables|Default|SetPlayerFound false))))

(event EventBeginPlay
  ;[1 1 1] On Start
  (Variables|Default|SetCurrentHealth (Variables|Default|GetMaxHealth))
  (bind _asai_hud (Utilities|Casting|CastToAI_HUD (UserInterface|GetUserWidgetObject (Variables|Default|GetWidget))))
  (Variables|/Game/GameBP/AI-BluePrints/HumanEnemies/AI_HUD.AI_HUD_C|SetOwner _asai_hud self)
  (CallFunction|SpawnAIWeapon))

(event EventITakeDamage
  (params (BodyPart :type Name :default "None") (Damage :type Float%20%28single-precision%29))
  ;[1 1 1] AI Take Damage From Player
  (Variables|Default|SetPlayerFound true)
  (if (Utilities|Name|Equal(Name) BodyPart "Head")
    (Variables|Default|SetCurrentHealth (- (Variables|Default|GetCurrentHealth) (* Damage 2.0)))
    (else
      (Variables|Default|SetCurrentHealth (- (Variables|Default|GetCurrentHealth) Damage))))
  (if (<= (Variables|Default|GetCurrentHealth) 0.0)
    (Utilities|FlowControl|DoOnce false
      (:Completed
        (Variables|Default|SetDead true)
        (Class|SkeletalMeshComponent|SetAllBodiesSimulatePhysics (Variables|Character|GetMesh) true)
        (Collision|SetCollisionEnabled (Variables|Collision|GetCapsuleComponent) "NoCollision")
        (Rendering|SetVisibility (Variables|Default|GetWidget) false false)
        (Components|DestroyComponent (Variables|Default|GetAlertSense))
        (Utilities|FlowControl|Delay 4.0)
        (CallFunction|SpawnItem)
        (Actor|DestroyActor (Variables|Default|GetWeaponBP))
        (Actor|DestroyActor)))))

(fn ConstructionScript)