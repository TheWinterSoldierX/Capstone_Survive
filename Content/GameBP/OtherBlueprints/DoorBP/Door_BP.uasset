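; Door Blueprint that the survivor opens and closes with an interaction input, requiring a key when locked.
; Box overlap toggles a custom-depth highlight and a DoorUI prompt, allowing opening if the door is unlocked or the player holds a key.
; OpenDoor and CloseDoor timelines swing the actor's yaw from its starting rotation.
; A DoOnce on opening deducts one player key and leaves the door permanently unlocked.
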(event OnComponentBeginOverlap(Box)
  (params (OverlappedComponent :type Primitive%20Component%20Object%20Reference) (OtherActor :type Actor%20Object%20Reference) (OtherComp :type Primitive%20Component%20Object%20Reference) (OtherBodyIndex :type Integer) (bFromSweep :type Boolean) (SweepResult :type Hit%20Result%20Structure%20%28by%20ref%29))
  (bind _asthird_person_survivor (Utilities|Casting|CastToThirdPersonSurvivor OtherActor))
  (Variables|Default|SetThirdPersonRef _asthird_person_survivor)
  (Rendering|SetRenderCustomDepth (Variables|Default|GetStaticMesh) true)
  (Rendering|SetVisibility (Variables|Default|GetWidget) true false)
  (if (Variables|Default|GetDoorUnlocked)
    (bind _asdoor_ui (Utilities|Casting|CastToDoorUI (UserInterface|GetUserWidgetObject (Variables|Default|GetWidget)) :!label _label))
    (Variables|/Game/GameBP/OtherBlueprints/DoorBP/DoorUI.DoorUI_C|SetKeyText _asdoor_ui "Open Door [ F ]")
    (Input|EnableInput (Game|GetPlayerController 0))
    (Variables|Default|SetCanOpen true)
    (elif (>= (Variables|/Game/GameBP/PlayerBlueprints/ThirdPersonSurvivor.ThirdPersonSurvivor_C|GetKey (Variables|Default|GetThirdPersonRef)) 1)
      (goto _label)
      (else
        (bind _asdoor_ui_2 (Utilities|Casting|CastToDoorUI (UserInterface|GetUserWidgetObject (Variables|Default|GetWidget))))
        (Variables|/Game/GameBP/OtherBlueprints/DoorBP/DoorUI.DoorUI_C|SetKeyText _asdoor_ui_2 "Locked")
        (Variables|Default|SetCanOpen false)))))

(event OnComponentEndOverlap(Box)
  (params (OverlappedComponent :type Primitive%20Component%20Object%20Reference) (OtherActor :type Actor%20Object%20Reference) (OtherComp :type Primitive%20Component%20Object%20Reference) (OtherBodyIndex :type Integer))
  (bind _asthird_person_survivor (Utilities|Casting|CastToThirdPersonSurvivor OtherActor))
  (Variables|Default|SetThirdPersonRef _asthird_person_survivor)
  (Rendering|SetRenderCustomDepth (Variables|Default|GetStaticMesh) false)
  (Rendering|SetVisibility (Variables|Default|GetWidget) false false)
  (Variables|Default|SetCanOpen false))

(event EventBeginPlay
  (Variables|Default|SetCurrentRotation (Transformation|GetActorRotation)))

(event Input|ActionEvents|InputActionItemInteraction
  (params (Key :type Key%20Structure))
  (:Pressed
    (if (Variables|Default|GetCanOpen)
      (if (Variables|Default|GetIsOpen)
        (bind _opendoor (Timeline|CloseDoor ReverseFromEnd)
          (:Update
            (Transformation|SetActorRelativeRotation (Math|Rotator|MakeRotator 0.0 0.0 (+ (.Yaw (Math|Rotator|BreakRotator (Variables|Default|GetCurrentRotation))) _opendoor)))
            (Variables|Default|SetIsOpen false)))
        (else
          (bind _opendoor_2 (Timeline|OpenDoor PlayFromStart)
            (:Update
              (Transformation|SetActorRelativeRotation (Math|Rotator|MakeRotator 0.0 0.0 (+ (.Yaw (Math|Rotator|BreakRotator (Variables|Default|GetCurrentRotation))) _opendoor_2)))
              (Variables|Default|SetIsOpen true)
              (Utilities|FlowControl|DoOnce false ; It will always want a key after you open door that's why you do Do once. It will always remain open after you open
                (:Completed
                  (bind _asthird_person_survivor (Utilities|Casting|CastToThirdPersonSurvivor (Game|GetPlayerCharacter 0)))
                  (bind _result (Math|Integer|DecrementInt (Variables|/Game/GameBP/PlayerBlueprints/ThirdPersonSurvivor.ThirdPersonSurvivor_C|GetKey _asthird_person_survivor))
                    (:%20%20
                      (Variables|/Game/GameBP/PlayerBlueprints/ThirdPersonSurvivor.ThirdPersonSurvivor_C|SetKey _asthird_person_survivor _result)
                      (Variables|Default|SetDoorUnlocked true))))))))))))

(fn ConstructionScript)