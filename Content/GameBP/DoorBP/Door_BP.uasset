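; Key-locked swinging door that a ThirdPersonSurvivor can open and close.
; Box overlap toggles a custom-depth highlight and a DoorUI prompt, showing "Locked" unless the survivor holds at least one key.
; With a key, it enables input and sets CanOpen, which gates the ItemInteraction press and clears on exit.
; Separate timelines swing the yaw from the BeginPlay rotation, with CloseDoor played in reverse; keys are not consumed.
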(event OnComponentBeginOverlap(Box)
  (params (OverlappedComponent :type Primitive%20Component%20Object%20Reference) (OtherActor :type Actor%20Object%20Reference) (OtherComp :type Primitive%20Component%20Object%20Reference) (OtherBodyIndex :type Integer) (bFromSweep :type Boolean) (SweepResult :type Hit%20Result%20Structure%20%28by%20ref%29))
  (bind _asthird_person_survivor (Utilities|Casting|CastToThirdPersonSurvivor OtherActor))
  (Variables|Default|SetThirdPersonRef _asthird_person_survivor)
  (Rendering|SetRenderCustomDepth (Variables|Default|GetStaticMesh) true)
  (Rendering|SetVisibility (Variables|Default|GetWidget) true false)
  (if (>= (Variables|/Game/GameBP/Blueprints/ThirdPersonSurvivor.ThirdPersonSurvivor_C|GetKey (Variables|Default|GetThirdPersonRef)) 1)
    (bind _asdoor_ui (Utilities|Casting|CastToDoorUI (UserInterface|GetUserWidgetObject (Variables|Default|GetWidget))))
    (Variables|/Game/GameBP/DoorBP/DoorUI.DoorUI_C|SetKeyText _asdoor_ui "Open Door [ F ]")
    (Input|EnableInput (Game|GetPlayerController 0))
    (Variables|Default|SetCanOpen true)
    (else
      (bind _asdoor_ui_2 (Utilities|Casting|CastToDoorUI (UserInterface|GetUserWidgetObject (Variables|Default|GetWidget))))
      (Variables|/Game/GameBP/DoorBP/DoorUI.DoorUI_C|SetKeyText _asdoor_ui_2 "Locked")
      (Variables|Default|SetCanOpen false))))

(event OnComponentEndOverlap(Box)
  (params (OverlappedComponent :type Primitive%20Component%20Object%20Reference) (OtherActor :type Actor%20Object%20Reference) (OtherComp :type Primitive%20Component%20Object%20Reference) (OtherBodyIndex :type Integer))
  (bind _asthird_person_survivor (Utilities|Casting|CastToThirdPersonSurvivor OtherActor))
  (Variables|Default|SetThirdPersonRef _asthird_person_survivor)
  (Rendering|SetRenderCustomDepth (Variables|Default|GetStaticMesh) false)
  (Rendering|SetVisibility (Variables|Default|GetWidget) false false)
  (Variables|Default|SetCanOpen false))

(event EventBeginPlay
  (Variables|Default|SetCurrentRotation (Transformation|GetActorRotation)))

(event Input|ActionEvents|InputActionItemInteraction
  (params (Key :type Key%20Structure :default "None"))
  (:Pressed
    (if (Variables|Default|GetCanOpen)
      (if (Variables|Default|GetIsOpen)
        (bind _opendoor (Timeline|CloseDoor ReverseFromEnd)
          (:Update
            (Transformation|SetActorRelativeRotation (Math|Rotator|MakeRotator 0.0 0.0 (+ (.Yaw (Math|Rotator|BreakRotator (Variables|Default|GetCurrentRotation))) _opendoor)))
            (Variables|Default|SetIsOpen false)
            (Development|PrintString "DoorClosed" true true "(R=1.000000,G=0.000000,B=0.000000,A=1.000000)")))
        (else
          (bind _opendoor_2 (Timeline|OpenDoor PlayFromStart)
            (:Update
              (Transformation|SetActorRelativeRotation (Math|Rotator|MakeRotator 0.0 0.0 (+ (.Yaw (Math|Rotator|BreakRotator (Variables|Default|GetCurrentRotation))) _opendoor_2)))
              (Variables|Default|SetIsOpen true)
              (Development|PrintString "DoorOpen" true true "(R=0.000000,G=1.000000,B=0.027462,A=1.000000)"))))))))

(fn ConstructionScript)